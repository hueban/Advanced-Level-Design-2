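; Elevator console actor that runs a scripted one-way ride from the bottom to the top floor.
; Its box trigger sets the third-person character's UsingElevator flag on overlap and clears it on exit.
; ElevatorGo closes the tagged bottom door, starts a tagged effect, then after timed delays teleports the player upward and opens the top door.
; The ride is faked with a fixed Z offset, and doors and effect are found by actor tag.
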(event `ElevatorGo`
  (bind _outactors (`GameplayStatics.GetAllActorsOfClassWithTag` "/Game/Interactables/ElevatorDoor.ElevatorDoor_C" "BottomElevator"))
  (`/Game/Interactables/ElevatorDoor.DoorClose` (`|GetArrayItem` _outactors))
  (`KismetSystemLibrary.Delay` 5.0)
  (bind _outactors_2 (`GameplayStatics.GetAllActorsOfClassWithTag` "/Game/Interactables/ElevatorEffect.ElevatorEffect_C" "BottomEffect"))
  (`/Game/Interactables/ElevatorEffect.ElevatorGo` (`|GetArrayItem` _outactors_2))
  (`KismetSystemLibrary.Delay` 11.0)
  (bind _asbp_third_person_character (cast `/Game/ThirdPerson/Blueprints/BP_ThirdPersonCharacter` (`GameplayStatics.GetPlayerCharacter` 0)))
  (`self.K2_SetActorLocation` _asbp_third_person_character (+ (`self.K2_GetActorLocation` _asbp_third_person_character) (0.0 0.0 6646.0)) false true)
  (bind _outactors_3 (`GameplayStatics.GetAllActorsOfClassWithTag` "/Game/Interactables/ElevatorDoor.ElevatorDoor_C" "TopDoor"))
  (`/Game/Interactables/ElevatorDoor.DoorOpen` (`|GetArrayItem` _outactors_3)))

(event `self.Box.OnComponentBeginOverlap`
  (params (OverlappedComponent :type "PrimitiveComponent Object Reference") (OtherActor :type "Actor Object Reference") (OtherComp :type "PrimitiveComponent Object Reference") (OtherBodyIndex :type Integer) (bFromSweep :type Boolean) (SweepResult :type "HitResult Structure (by ref)"))
  (bind _asbp_third_person_character (cast `/Game/ThirdPerson/Blueprints/BP_ThirdPersonCharacter` OtherActor))
  (set `/Game/ThirdPerson/Blueprints/BP_ThirdPersonCharacter.UsingElevator` true _asbp_third_person_character))

(event `self.Box.OnComponentEndOverlap`
  (params (OverlappedComponent :type "PrimitiveComponent Object Reference") (OtherActor :type "Actor Object Reference") (OtherComp :type "PrimitiveComponent Object Reference") (OtherBodyIndex :type Integer))
  (bind _asbp_third_person_character (cast `/Game/ThirdPerson/Blueprints/BP_ThirdPersonCharacter` OtherActor))
  (set `/Game/ThirdPerson/Blueprints/BP_ThirdPersonCharacter.UsingElevator` false _asbp_third_person_character))

(fn `UserConstructionScript`)