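; BP_QuestTerminal is an interactable terminal that grants the player an upgrade choice and a quest.
; Box overlap toggles the character's AcessingTerminal flag.
; The Animation event plays the BrainJacking timeline, swinging two cubes oppositely and lowering the Interface.
; When the track first hits 1.0 it pauses the game and opens the upgrade menu, guarded by UpgradeChosen; timeline completion calls GetQuest on the character.
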(event `self.Box.OnComponentBeginOverlap`
  (params (OverlappedComponent :type "PrimitiveComponent Object Reference") (OtherActor :type "Actor Object Reference") (OtherComp :type "PrimitiveComponent Object Reference") (OtherBodyIndex :type Integer) (bFromSweep :type Boolean) (SweepResult :type "HitResult Structure (by ref)"))
  (bind _asbp_third_person_character (cast `/Game/ThirdPerson/Blueprints/BP_ThirdPersonCharacter` OtherActor))
  (set `/Game/ThirdPerson/Blueprints/BP_ThirdPersonCharacter.AcessingTerminal` true _asbp_third_person_character))

(event `self.Box.OnComponentEndOverlap`
  (params (OverlappedComponent :type "PrimitiveComponent Object Reference") (OtherActor :type "Actor Object Reference") (OtherComp :type "PrimitiveComponent Object Reference") (OtherBodyIndex :type Integer))
  (bind _asbp_third_person_character (cast `/Game/ThirdPerson/Blueprints/BP_ThirdPersonCharacter` OtherActor))
  (set `/Game/ThirdPerson/Blueprints/BP_ThirdPersonCharacter.AcessingTerminal` false _asbp_third_person_character))

(event `Animation`
  (bind _interface (`self.Interface`))
  (bind (_relativelocation_x _relativelocation_y) (`KismetMathLibrary.BreakVector` (`SceneComponent.RelativeLocation` _interface)))
  (bind (_direction _newtrack_0) (`Timeline|BrainJacking`)
    (:`Update`
      (if (`self.UpgradeChosen`)
        (bind _returnvalue (`KismetMathLibrary.Lerp` 0.0 20.0 _newtrack_0))
        (`SceneComponent.K2_SetRelativeRotation` (`self.Cube2`) (`KismetMathLibrary.MakeRotator` 0.0 0.0 (* _returnvalue -1.0)) false false :!label _label)
        (`SceneComponent.K2_SetRelativeRotation` (`self.Cube1`) (`KismetMathLibrary.MakeRotator` 0.0 0.0 _returnvalue) false false)
        (`SceneComponent.K2_SetRelativeLocation` _interface (`KismetMathLibrary.MakeVector` _relativelocation_x _relativelocation_y (`KismetMathLibrary.Lerp` 52.0 35.0 _newtrack_0)) false false)
        (elif (== _newtrack_0 1.0)
          (`GameplayStatics.SetGamePaused` true)
          (bind _asbp_third_person_character (cast `/Game/ThirdPerson/Blueprints/BP_ThirdPersonCharacter` (`GameplayStatics.GetPlayerCharacter` 0)))
          (`/Game/ThirdPerson/Blueprints/BP_ThirdPersonCharacter.UpgradeMenu` _asbp_third_person_character)
          (set `self.UpgradeChosen` true)
          (else
            (goto _label)))))
    (:`Finished`
      (bind _asbp_third_person_character_2 (cast `/Game/ThirdPerson/Blueprints/BP_ThirdPersonCharacter` (`GameplayStatics.GetPlayerCharacter` 0)))
      (`/Game/ThirdPerson/Blueprints/BP_ThirdPersonCharacter.GetQuest` _asbp_third_person_character_2))))

(fn `UserConstructionScript`)