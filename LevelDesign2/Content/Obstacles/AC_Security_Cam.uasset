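; Security camera obstacle that detects the player and can sweep its yaw between two limits via a timeline.
; A visible player entering its capsule marks it as seeing and turns the spotlight to the alert color, which reverts after a delay on exit.
; While the player is visible, Tick raises or slowly drains AlertValue through short Delays, printing each change.
; At full alert, it sets IsDetected on the player character.
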(event `CheckForPlayer`
  (bind _returnvalue (`GameplayStatics.GetPlayerCharacter` 0))
  (bind _asbp_third_person_character (cast `/Game/ThirdPerson/Blueprints/BP_ThirdPersonCharacter` _returnvalue))
  (if (`/Game/ThirdPerson/Blueprints/BP_ThirdPersonCharacter.IsPlayerVisible` _asbp_third_person_character)
    (if (>= (`self.AlertValue`) 100.0)
      (bind _asbp_third_person_character_2 (cast `/Game/ThirdPerson/Blueprints/BP_ThirdPersonCharacter` _returnvalue))
      (set `/Game/ThirdPerson/Blueprints/BP_ThirdPersonCharacter.IsDetected` true _asbp_third_person_character_2)
      (elif (`self.SeeingPlayer`)
        (`KismetSystemLibrary.Delay` 0.01)
        (`self.Affect AlertValue` 2.0)
        (elif (not (<= (`self.AlertValue`) 0.0))
          (`KismetSystemLibrary.Delay` 0.01)
          (`self.Affect AlertValue` -0.5))))))

(event `self.ReceiveBeginPlay`
  (if (`self.Rotating`)
    (`KismetSystemLibrary.Delay` (`self.MoveDelay`))
    (`self.StartMove`)))

(event `Affect AlertValue`
  (params (Amount :type "Float (double-precision)"))
  (bind _output_get (set `self.AlertValue` (+ (`self.AlertValue`) Amount)))
  (`KismetSystemLibrary.PrintString` (`KismetStringLibrary.Conv_DoubleToString` _output_get)))

(event `self.Capsule.OnComponentBeginOverlap`
  (params (OverlappedComponent :type "PrimitiveComponent Object Reference") (OtherActor :type "Actor Object Reference") (OtherComp :type "PrimitiveComponent Object Reference") (OtherBodyIndex :type Integer) (bFromSweep :type Boolean) (SweepResult :type "HitResult Structure (by ref)"))
  (bind _asbp_third_person_character (cast `/Game/ThirdPerson/Blueprints/BP_ThirdPersonCharacter` OtherActor))
  (if (`/Game/ThirdPerson/Blueprints/BP_ThirdPersonCharacter.IsPlayerVisible` _asbp_third_person_character)
    (set `self.SeeingPlayer` true)
    (`LightComponent.SetLightColor` (`self.SpotLight`) (`self.AlertColor`) true)))

(event `self.ReceiveTick`
  (params (DeltaSeconds :type "Float (single-precision)"))
  (`self.CheckForPlayer`))

(event `StartMove`
  (bind (_returnvalue_roll _returnvalue_pitch) (`KismetMathLibrary.BreakRotator` (`self.K2_GetActorRotation`)))
  (bind (_direction _rotationcurve) (`Timeline|Rotation`)
    (:`Update`
      (`self.K2_SetActorRelativeRotation` (`KismetMathLibrary.MakeRotator` _returnvalue_roll _returnvalue_pitch (`KismetMathLibrary.Lerp` (`self.MinDeg`) (`self.MaxDeg`) _rotationcurve))))))

(event `self.Capsule.OnComponentEndOverlap`
  (params (OverlappedComponent :type "PrimitiveComponent Object Reference") (OtherActor :type "Actor Object Reference") (OtherComp :type "PrimitiveComponent Object Reference") (OtherBodyIndex :type Integer))
  (set `self.SeeingPlayer` false)
  (`KismetSystemLibrary.Delay` 3.0)
  (`LightComponent.SetLightColor` (`self.SpotLight`) (`self.IdleColor`) true))

(fn `UserConstructionScript`)